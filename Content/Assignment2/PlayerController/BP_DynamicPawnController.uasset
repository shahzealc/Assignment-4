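; BP_DynamicPawnController is a controller Blueprint that shows a pawn's attributes as on-screen debug text.
; Its DisplayAttributes event takes a PawnAttributeAsset and prints its Health, Speed and JumpHeight as labeled strings, with JumpHeight given a custom text color.
; BeginPlay, Tick and the construction script are empty, and nothing in this Blueprint calls DisplayAttributes.
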(event `self.ReceiveBeginPlay`)

(event `self.DisplayAttributes`
  (params (PawnAttributeAsset :type "PawnAttributeAsset Object Reference"))
  (`KismetSystemLibrary.PrintString` (`KismetStringLibrary.Concat_StrStr` "Health : " (`KismetStringLibrary.Conv_IntToString` (`PawnAttributeAsset.Health` PawnAttributeAsset))) true true (struct :`R` 0.221412 :`G` 1.0 :`B` 0.008226 :`A` 1.0))
  (`KismetSystemLibrary.PrintString` (`KismetStringLibrary.Concat_StrStr` "Speed : " (`KismetStringLibrary.Conv_DoubleToString` (`PawnAttributeAsset.Speed` PawnAttributeAsset))) true true (struct :`R` 1.0 :`G` 0.891706 :`B` 0.002064 :`A` 1.0))
  (`KismetSystemLibrary.PrintString` (`KismetStringLibrary.Concat_StrStr` "JumpHeight : " (`KismetStringLibrary.Conv_DoubleToString` (`PawnAttributeAsset.JumpHeight` PawnAttributeAsset))) true true (struct :`R` 0.751235 :`G` 0.01967 :`B` 1.0 :`A` 1.0)))

(fn `UserConstructionScript`)