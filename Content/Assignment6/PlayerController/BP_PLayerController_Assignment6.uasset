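; Player controller that drives a mesh generation tool through an on-screen UI.
; It binds widget dispatchers for shape, radius and dimension changes to update the selection area, and left click toggles the MoveActor flag.
; Generate requests pass the instance count, selection actor's location, scaled size and shape to BP_MeshGenerator.
; Progress events update the widget's progress bar, then hide it and reveal the Generate control.
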(event `self.ReceiveBeginPlay`
  (bind _meshgenerationui_ref (`self.MeshGenerationUI_Ref`))
  ;[1 1 1] Creating Widget
  (bind _returnvalue (`|CreateWidget` "/Game/Assignment6/User_Widget/W_MeshGenerationUI.W_MeshGenerationUI_C"))
  (bind _output_get (set `self.MeshGenerationUI_Ref` _returnvalue))
  (`UserWidget.AddToViewport` _output_get 0)
  (set `self.bShowMouseCursor` true)
  ;[1 1 1] On Shape Change
  (add `/Game/Assignment6/User_Widget/W_MeshGenerationUI.OnShapeChange` _meshgenerationui_ref (delegate `OnShapeChange_Event`))
  ;[1 1 1] On Radius Change
  (add `/Game/Assignment6/User_Widget/W_MeshGenerationUI.OnRadiusChange` _meshgenerationui_ref (delegate `OnRadiusChange_Event`))
  ;[1 1 1] On Dimention Change
  (add `/Game/Assignment6/User_Widget/W_MeshGenerationUI.OnDimentionChange` _meshgenerationui_ref (delegate `OnDimentionChange_Event`))
  ;[1 1 1] Generate Meshes
  (add `/Game/Assignment6/User_Widget/W_MeshGenerationUI.OnGenerateMesh` _meshgenerationui_ref (delegate `OnGenerateMesh_Event`)))

(event `OnShapeChange_Event`
  (params (ShapeToToggle :type String))
  ;[1 1 1] On Shape Change
  (`self.ToggleSelectionArea` ShapeToToggle))

(event `OnRadiusChange_Event`
  (params (Radius :type "Float (double-precision)"))
  ;[1 1 1] On Radius Change
  (`self.ChangeRadiusAndDimention` (`KismetMathLibrary.Conv_DoubleToVector` Radius)))

(event `OnDimentionChange_Event`
  (params (Length :type "Float (double-precision)") (Width :type "Float (double-precision)") (Height :type "Float (double-precision)"))
  ;[1 1 1] On Dimention Change
  (`self.ChangeRadiusAndDimention` (`KismetMathLibrary.MakeVector` Length Width Height)))

(event `OnGenerateMesh_Event`
  (params (Instances :type Integer))
  (bind _selectionactor (`self.SelectionActor`))
  ;[1 1 1] Generate Meshes
  (bind _returnvalue (`GameplayStatics.GetActorOfClass` "/Game/Assignment6/MeshGeneratorActor/BP_MeshGenerator_.BP_MeshGenerator__C"))
  (bind _output_get (set `self.MeshGenerator_Ref` _returnvalue))
  (`MeshGenerator.GenerateStaticMeshes` _output_get Instances (`self.K2_GetActorLocation` _selectionactor) (* (`self.GetActorScale3D` _selectionactor) (100.0 100.0 100.0)) (`/Game/Assignment6/User_Widget/W_MeshGenerationUI.isBoxSelected` (`self.MeshGenerationUI_Ref`))))

(event `Key|LeftMouseButton`
  (params (Key :type "Key Structure"))
  ;[1 1 1] LeftClick Event
  (:`Pressed`
    (if (`self.MoveActor`)
      (set `self.MoveActor` false)
      (else
        (set `self.MoveActor` true)))))

(event `ProgressBarChange`
  (params (`Current Progress` :type "Float (double-precision)"))
  ;[1 1 1] ProgressBar Change
  (set `/Game/Assignment6/User_Widget/W_MeshGenerationUI.ProgressBarValue` `Current Progress` (`self.MeshGenerationUI_Ref`)))

(event `RemoveProgressBar`
  (bind _meshgenerationui_ref (`self.MeshGenerationUI_Ref`))
  ;[1 1 1] Remove ProgressBar
  (`Widget.SetVisibility` (`/Game/Assignment6/User_Widget/W_MeshGenerationUI.ProgressMenu` _meshgenerationui_ref) "Hidden")
  (`Widget.SetVisibility` (`/Game/Assignment6/User_Widget/W_MeshGenerationUI.GenerateMeshes` _meshgenerationui_ref) "Visible"))

(fn `UserConstructionScript`)